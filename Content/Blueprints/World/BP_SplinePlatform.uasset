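; BP_SplinePlatform is a platform that moves along a spline from the start of play, driven by a timeline with optional looping.
; Timeline updates map alpha to distance along the spline, setting the scene component's world location with sweep and optionally matching spline rotation.
; When reversing is enabled, a FlipFlop on timeline completion alternates between reverse and forward playback.
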(event EventBeginPlay
  (Components|Timeline|SetPlayRate (Variables|Default|GetMoveTimeline) (|(1/{8EF6F62A-42D8-7EDE-FF05-99B379919D8A})))
  (Components|Timeline|SetLooping (Variables|Default|GetMoveTimeline) (Variables|Default|GetCanLoop))
  (Audio|Components|Audio|Play (Variables|Default|GetMoveTimeline)))

(fn ConstructionScript)