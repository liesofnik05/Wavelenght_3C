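; BP_DynamicLadder is a procedurally built ladder whose height follows the Z value of its Handle vector.
; The construction script converts that height into whole 100-unit segments, then scales and repositions the Left and Right side meshes to span them.
; It then loops over the segment count, adding one rotated, thinly scaled static mesh component as a rung every 100 units.
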(fn ConstructionScript
  (bind _handle (Variables|Default|GetHandle))
  (bind _returnvalue (/ (.z _handle) 1e+02))
  (bind _returnvalue_2 (Math|Float|Floor _returnvalue))
  (bind _returnvalue_3 (* _returnvalue_2 50))
  (bind _returnvalue_4 (- _returnvalue_3 50))
  (bind _returnvalue_5 (Math|Conversions|ToFloat(Integer) _returnvalue_4))
  (Transformation|SetRelativeScale3D (Variables|Default|GetRight) (Math|Vector|MakeVector 0.1 0.1 (Math|Conversions|ToFloat(Integer) _returnvalue_2)))
  (Transformation|SetRelativeLocation (Variables|Default|GetRight) (Math|Vector|MakeVector 45.0 0.0 _returnvalue_5) false false)
  (Transformation|SetRelativeLocation (Variables|Default|GetLeft) (Math|Vector|MakeVector -45.0 0.0 _returnvalue_5) false false)
  (for _index (range 0 (- _returnvalue_2 1))
    (AddComponent|AddStaticMeshComponent false (Math|Transform|MakeTransform (Math|Vector|MakeVector 0.0 0.0 (Math|Conversions|ToFloat(Integer) (* _index 100))) "90.000000,0.000000,0.000000" "0.100000,0.100000,0.900000"))))