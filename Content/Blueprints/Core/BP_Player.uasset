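; Player character with camera-relative movement, look, multi-jump and a cooldown-limited dash.
; A CanMove lock counter, checked by CanMoveState, gates look, move and jump during dashes and after damage.
; Landing refills jumps, while leaving the ground uses a retriggerable delay as coyote time before consuming one.
; Dash briefly zeroes gravity, braking and velocity to launch along control yaw; any damage hides and freezes the character.
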(event Input|EnhancedActionEvents|EnhancedInputActionIA_Look
  (params (ActionValue :type Vector%202D%20Structure) (ElapsedSeconds :type Float%20%28double-precision%29) (TriggeredSeconds :type Float%20%28double-precision%29) (InputAction :type Input%20Action%20Object%20Reference :default "/Game/Inputs/IA_Look.IA_Look"))
  (bind (_x _y) (Math|Vector2D|BreakVector2D ActionValue))
  (Utilities|CanMoveState
    (:Can%20Move
      (Pawn|Input|AddControllerYawInput _x)
      (Pawn|Input|AddControllerPitchInput _y))))

(event Input|EnhancedActionEvents|EnhancedInputActionIA_Move
  (params (ActionValue :type Vector%202D%20Structure) (ElapsedSeconds :type Float%20%28double-precision%29) (TriggeredSeconds :type Float%20%28double-precision%29) (InputAction :type Input%20Action%20Object%20Reference :default "/Game/Inputs/IA_Move.IA_Move"))
  (bind (_x _y) (Math|Vector2D|BreakVector2D ActionValue))
  (Utilities|CanMoveState
    (:Can%20Move
      (Pawn|Input|AddMovementInput (Math|Vector|GetRightVector (Math|Rotator|MakeRotator 0.0 0.0 (.yaw (Pawn|GetControlRotation :!class /Script/Engine.Pawn)))) _x false)
      (Pawn|Input|AddMovementInput (Math|Vector|GetForwardVector (Math|Rotator|MakeRotator 0.0 0.0 (.yaw (Pawn|GetControlRotation :!class /Script/Engine.Pawn)))) _y false))))

(event Input|EnhancedActionEvents|EnhancedInputActionIA_Jump
  (params (ActionValue :type Boolean) (ElapsedSeconds :type Float%20%28double-precision%29) (TriggeredSeconds :type Float%20%28double-precision%29) (InputAction :type Input%20Action%20Object%20Reference :default "/Game/Inputs/IA_Jump.IA_Jump"))
  (:Started
    (Utilities|CanMoveState
      (:Can%20Move
        (if (Math|Conversions|ToBoolean(Integer) (Variables|Default|GetCurrentJumpCount))
          (Math|Integer|DecrementInt (Variables|Default|GetCurrentJumpCount)
            (:%20%20
              (Character|Jump)))))))
  (:Completed
    (Character|StopJumping)))

(event Input|EnhancedActionEvents|EnhancedInputActionIA_Dash
  (params (ActionValue :type Boolean) (ElapsedSeconds :type Float%20%28double-precision%29) (TriggeredSeconds :type Float%20%28double-precision%29) (InputAction :type Input%20Action%20Object%20Reference :default "/Game/Inputs/IA_Dash.IA_Dash"))
  (bind _returnvalue (Pawn|GetControlRotation :!class /Script/Engine.Pawn))
  (bind _charactermovement (Variables|Character|GetCharacterMovement))
  (bind _charactermovement_2 (Variables|Character|GetCharacterMovement))
  (bind _returnvalue_2 (Math|Vector|GetForwardVector (Math|Rotator|MakeRotator 0.0 0.0 (.yaw _returnvalue))))
  (:Started
    (Utilities|DoOncewithAfter :!label _label
      (:Once
        (Utilities|FlowControl|Sequence
          (:then_0
            (Math|Integer|IncrementInt (Variables|Default|GetCanMove)
              (:%20%20
                (Utilities|FlowControl|DelayUntilNextTick)
                (Utilities|FlowControl|Sequence
                  (:then_0
                    (Variables|/Script/Engine.CharacterMovementComponent|SetGravityScale _charactermovement_2 0.0)
                    (Variables|/Script/Engine.CharacterMovementComponent|SetBrakingDecelerationFalling _charactermovement_2 0.0)
                    (Variables|/Script/Engine.CharacterMovementComponent|SetBrakingDecelerationWalking _charactermovement_2 0.0)
                    (Variables|/Script/Engine.MovementComponent|SetVelocity _charactermovement_2 "0, 0, 0")
                    (Variables|/Script/Engine.CharacterMovementComponent|SetRotationRate _charactermovement_2 "0.000000,-1.000000,0.000000"))
                  (:then_1
                    (Pawn|Input|AddMovementInput _returnvalue_2 1.0 false)
                    (Character|LaunchCharacter (* _returnvalue_2 3e+03) false false))))))
          (:then_1
            (Utilities|FlowControl|Delay 0.2)
            (Variables|Rendering|GetbHidden
              (:then
                _)
              (:else
                (Variables|/Script/Engine.CharacterMovementComponent|SetGravityScale (Variables|Character|GetCharacterMovement) (Variables|Default|GetGravityScaleRef))))
            (Variables|/Script/Engine.CharacterMovementComponent|SetBrakingDecelerationFalling _charactermovement (Variables|Default|GetBrakingDeceleration))
            (Variables|/Script/Engine.CharacterMovementComponent|SetBrakingDecelerationWalking _charactermovement (Variables|Default|GetBrakingDeceleration))
            (Variables|/Script/Engine.CharacterMovementComponent|SetRotationRate _charactermovement "0.000000,500.000000,0.000000")
            (Math|Integer|DecrementInt (Variables|Default|GetCanMove)
              (:%20%20
                (Utilities|FlowControl|Delay 3.0)
                (goto _label Reset)))))))))

(event EventOnMovementModeChanged
  (params (PrevMovementMode :type EMovementMode%20Enum :default "MOVE_None") (NewMovementMode :type EMovementMode%20Enum :default "MOVE_None") (PrevCustomMode :type Byte :default 0) (NewCustomMode :type Byte :default 0))
  (if (AI|Components|NavMovement|IsMovingonGround (Variables|Character|GetCharacterMovement))
    (Variables|Default|SetCurrentJumpCount (- (Variables|Default|GetJumpMaxCount) 1))
    (goto _label Reset)
    (else
      (Utilities|FlowControl|DoOnce false :!label _label
        (:Completed
          (Utilities|FlowControl|RetriggerableDelay 0.2)
          (if (and (not (AI|Components|NavMovement|IsMovingonGround (Variables|Character|GetCharacterMovement))) (== (Variables|Default|GetCurrentJumpCount) (- (Variables|Default|GetJumpMaxCount) 1)))
            (Math|Integer|DecrementInt (Variables|Default|GetCurrentJumpCount))))))))

(event Game|Damage|EventAnyDamage
  (params (Damage :type Float%20%28single-precision%29) (DamageType :type Damage%20Type%20Object%20Reference) (InstigatedBy :type Controller%20Object%20Reference) (DamageCauser :type Actor%20Object%20Reference))
  (bind _charactermovement (Variables|Character|GetCharacterMovement))
  (Math|Integer|IncrementInt (Variables|Default|GetCanMove)
    (:%20%20
      (Rendering|SetActorHiddenInGame true)
      (Utilities|FlowControl|DelayUntilNextTick)
      (Variables|/Script/Engine.CharacterMovementComponent|SetGravityScale _charactermovement 0.0)
      (Variables|/Script/Engine.MovementComponent|SetVelocity _charactermovement "0, 0, 0"))))

(event EventBeginPlay
  (Variables|Default|SetJumpMaxCount (+ (Variables|Default|GetCurrentJumpCount) 1))
  (Variables|Default|SetJumpMaxHoldTime 0.2))

(fn ConstructionScript)